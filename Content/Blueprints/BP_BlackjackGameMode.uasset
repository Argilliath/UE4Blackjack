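; Blackjack game mode that drives a round through a state machine, from betting and dealing through player choices, the dealer's play and payout.
; Each state change runs that phase's logic, such as blackjack and bust checks, often advancing to the next state, then notifies the game UI.
; Players with deals remaining receive newly spawned cards, and once all are done play passes to the dealer.
; A lazily cached, cast UI reference also forwards pause presses.
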(event EventOnGameStateChanged
  (params (OldState :type EBlackjackGameState%20Enum :default "RoundStart"))
  (Utilities|FlowControl|Sequence
    (:then_0
      (switch Utilities|FlowControl|Switch|SwitchonEBlackjackGameState (Variables|Default|GetCurrentGameState)
        (:RoundStart
          (Class|BlackjackGameMode|ChangeGameState "WaitForBet"))
        (:InitialShuffle
          (Class|BlackjackGameMode|ChangeGameState "InitialDeal"))
        (:InitialDeal
          (Class|BlackjackGameMode|ProcessInitialDeal)
          (Class|BlackjackGameMode|CheckforDealerBlackjack))
        (:WaitForCardDeal
          (if (Class|BlackjackGameMode|AreAllPlayersDone)
            (Class|BlackjackGameMode|ChangeGameState "DealerDeal")
            (else
              (CallFunction|DealPlayersCards)
              (Class|BlackjackGameMode|CheckforPlayersBust)
              (if (Class|BlackjackGameMode|AreAllPlayersDone)
                (Class|BlackjackGameMode|ChangeGameState "DealerDeal")
                (else
                  (Class|BlackjackGameMode|ChangeGameState "WaitForPlayerChoice"))))))
        (:DealerDeal
          (Class|BlackjackGameMode|ProcessDealersPlay)
          (Class|BlackjackGameMode|CheckRoundResults)
          (Class|BlackjackGameMode|ChangeGameState "RoundResults"))
        (:RoundResults
          (Class|BlackjackGameMode|CollectBetMoney))))
    (:then_1
      (Default|OnGameStateChanged (CallFunction|GetCachedGameUI) (Variables|Default|GetCurrentGameState) OldState))))

(fn ConstructionScript)

(fn GetCachedGameUI
  (Utilities|IsValid (Variables|Default|GetCachedGameUI)
    (:Is%20Valid
      (return (Variables|Default|GetCachedGameUI)))
    (:Is%20Not%20Valid
      (bind _asgame_ui (Utilities|Casting|CastToGameUI (Variables|Default|GetGameUI)))
      (bind _output_get (Variables|Default|SetCachedGameUI _asgame_ui))
      (return _output_get))))

(fn DealPlayersCards
  (for (_array_element _array_index) (Variables|Default|GetPlayersInfo)
    (if (> (.RemainingDealsLeft (Utilities|Struct|BreakPlayerInfo _array_element)) 0)
      (bind _returnvalue (Class|BlackjackGameMode|SpawnNextCard))
      (Class|BlackjackGameMode|GiveCard _array_index _returnvalue))))

(fn CallPause
  (bind _cachedgameui (CallFunction|GetCachedGameUI))
  (Utilities|IsValid _cachedgameui
    (:Is%20Valid
      (Default|OnPausePressed _cachedgameui))))